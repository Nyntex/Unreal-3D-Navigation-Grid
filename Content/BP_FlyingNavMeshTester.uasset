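; Test pawn for 3D flying navigation that keeps sending itself to random movable positions on a nav grid.
; BeginPlay starts an async 3D move, then issues a new one every six seconds from the Started output, without waiting for completion.
; Move results are printed for debugging.
; Unused steering helpers, a FlyingMovement random-move event and disconnected experiments, including a retry-on-finish loop, remain alongside the active loop.
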(event Custom|MoveToRandomPosition
  (Utilities|FlowControl|Delay 0.2)
  (Default|MovetoRandomPosition (Variables|Default|GetFlying%20Movement)))

(event EventBeginPlay
  (bind _returnvalue (Transformation|GetActorLocation))
  (bind _returnvalue_2 (Transformation|GetActorLocation))
  (bind _returnvalue_3 (Class|HeightNavigationVolume|EvaluateNavGrid _returnvalue _returnvalue))
  (bind _returnvalue_4 (Class|HeightNavigationVolume|EvaluateNavGrid _returnvalue_2 _returnvalue_2))
  (Utilities|IsValid _returnvalue_4 :!label _label
    (:Is%20Valid
      (Class|LAMovetoLocationorActor3D|MovetoActororLocation3D (Class|HeightNavigationVolume|GetRandomMovablePosition _returnvalue_4)
        (:OnStarted
          (Utilities|FlowControl|Delay 6.0 :!label _label_2)
          (Utilities|IsValid _returnvalue_3
            (:Is%20Valid
              (Class|LAMovetoLocationorActor3D|MovetoActororLocation3D (Class|HeightNavigationVolume|GetRandomMovablePosition _returnvalue_3)
                (:OnStarted
                  (Utilities|FlowControl|Delay 6.0 :!label _label_3)
                  (goto _label))
                (:OnCanceled
                  (Development|PrintString "Canceled"))
                (:OnCompleted
                  (Development|PrintString "Completed"))
                (:OnFailed
                  (Development|PrintString "Failed")))
              (for _array_element (Utilities|Array|MakeArray "ObjectTypeQuery1" "ObjectTypeQuery2")
                (Development|PrintString (Utilities|String|ToString(Integer) (Math|Conversions|ToInteger(Byte) _array_element)))))
            (:Is%20Not%20Valid
              (goto _label_3))))
        (:OnCanceled
          (Development|PrintString "Canceled"))
        (:OnCompleted
          (Development|PrintString "Completed"))
        (:OnFailed
          (Development|PrintString "Failed"))))
    (:Is%20Not%20Valid
      (goto _label_2))))

(event Collision|EventActorBeginOverlap
  (params (OtherActor :type Actor%20Object%20Reference)))

(event EventTick
  (params (DeltaSeconds :type Float%20%28single-precision%29)))

(fn ConstructionScript)

(fn RotatetoMoveDirection
  (params (Direction :type Vector))
  (bind _returnvalue (Transformation|GetActorLocation))
  (Transformation|SetActorRotation (Math|Rotator|MakeRotator 0.0 0.0 (.yaw (Math|Rotator|FindLookatRotation _returnvalue (+ Direction _returnvalue))))))

(fn IsCloseEnough
  (return (<= (Math|Vector|Distance(Vector) (Utilities|Array|Get(acopy) (Variables|Old|GetPath)) (Transformation|GetActorLocation)) 2.5e+02)))

(fn GetDirectionPosition
  (params (Position :type Vector))
  (return (Math|Vector|Normalize (- Position (Transformation|GetActorLocation)))))

(fn IsMoveInsideNavMesh
  (return (Class|HeightNavigationVolume|IsInsideVolume (Variables|Old|GetNavMesh) (+ (Transformation|GetActorLocation) (* (Variables|Old|GetCurrentDirection) 1e+02)))))

(fn MovetoPosition
  (params (Position :type Vector))
  (if (Class|KismetMathLibrary|NotEqualExactlyVectorVector Position (Transformation|GetActorLocation))
    (Pawn|Input|AddMovementInput (CallFunction|GetDirectionPosition Position) 1.0 false)
    (return)))

(fn IsBelowThreshold
  (params (Threshold :type Float%20%28double-precision%29))
  (return (<= (Math|Vector|Distance(Vector) (Variables|Old|GetLastPositionToMoveTo) (Transformation|GetActorLocation)) Threshold)))