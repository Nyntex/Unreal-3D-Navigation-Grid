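; Pawn component for flying navigation that moves its owner to positions, actor locations or random points within a HeightNavigationVolume.
; Move commands go straight when a visibility trace is clear, otherwise follow a path from the volume enclosing start and goal.
; Tick feeds movement input toward the current waypoint, snapping onto the final one when close.
; A looping delayed trace switches between direct flight and re-pathing as line of sight changes.
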(event Custom|MoveToActor
  (params (Actor :type Actor%20Object%20Reference))
  ;[1 1 1] Movement Commands
  (Utilities|IsValid Actor
    (:Is%20Valid
      (CallFunction|MovetoNewPosition (Transformation|GetActorLocation Actor)))))

(event Custom|DirectPathLoop
  (bind _ownerpawn (Variables|Default|GetOwnerPawn))
  ;[1 1 1] Movement Loop
  (Utilities|FlowControl|DoOnce false :!label _label
    (:Completed
      (if (Variables|Default|GetFinishedMovment)
        _
        (else
          (Variables|Default|SetPreviousCheckDirectPathToTarget (Variables|Default|GetDirectPathToTarget))
          (bind (_outhit _returnvalue) (Collision|LineTraceByChannel (Transformation|GetActorLocation _ownerpawn) (Variables|Default|GetTargetPosition) "TraceTypeQuery1" false (Utilities|Array|MakeArray _ownerpawn) "ForDuration" true "(R=1.000000,G=0.000000,B=0.000000,A=1.000000)" "(R=0.000000,G=1.000000,B=0.000000,A=1.000000)" 0.5))
          (if (and _returnvalue (Utilities|Operators|NotEqual(!=) (.Location (Collision|BreakHitResult _outhit)) (Variables|Default|GetTargetPosition) 1e+01))
            (Variables|Default|SetDirectPathToTarget false)
            (else
              (Variables|Default|SetDirectPathToTarget true)
              (Utilities|FlowControl|Delay 1.0)))))
      (Utilities|FlowControl|Delay 0.5)
      (Utilities|FlowControl|Sequence
        (:then_0
          (goto _label Reset))
        (:then_1
          (CallFunction|DirectPathLoop))))))

(event Custom|MoveToNewPosition
  (params (GoalPosition :type Vector))
  (bind _ownerpawn (Variables|Default|GetOwnerPawn))
  ;[1 1 1] Movement Commands
  (Utilities|IsValid (CallFunction|EvaluateCurrentNavGrid (Transformation|GetActorLocation (Variables|Default|GetOwnerPawn)) GoalPosition)
    (:Is%20Valid
      (bind _output_get (Variables|Default|SetTargetPosition GoalPosition))
      (bind (_outhit _returnvalue) (Collision|LineTraceByChannel (Transformation|GetActorLocation _ownerpawn) _output_get "TraceTypeQuery1" false (Utilities|Array|MakeArray _ownerpawn) "None"))
      (if (and _returnvalue (Utilities|Operators|NotEqual(!=) (.Location (Collision|BreakHitResult _outhit)) GoalPosition 1e+01))
        (bind (_path _success) (CallFunction|GetNewPathtoPosition GoalPosition))
        (if _success
          (bind _output_get_2 (Variables|Default|SetPath _path))
          (bind _output_get_3 (Variables|Default|SetFinishedMovment (Utilities|Array|IsEmpty _output_get_2)))
          (if _output_get_3
            (CallFunction|StopMovement false :!label _label)
            (else
              (Variables|Default|SetpathCounter 0)
              (Variables|Default|SetLastPositionToMoveTo (Utilities|Array|Get(acopy) (Variables|Default|GetPath)))
              (Variables|Default|SetDirectPathToTarget false)))
          (else
            (goto _label)))
        (else
          (Variables|Default|SetPath (Utilities|Array|MakeArray GoalPosition))
          (Variables|Default|SetLastPositionToMoveTo GoalPosition)
          (Variables|Default|SetFinishedMovment false)
          (Variables|Default|SetpathCounter 0)
          (Variables|Default|SetDirectPathToTarget true))))
    (:Is%20Not%20Valid
      (CallFunction|StopMovement true))))

(event Custom|StopMovement
  (params (Instant :type Boolean))
  ;[1 1 1] Movement Commands
  (Class|Pawn|ConsumeMovementInputVector (Variables|Default|GetOwnerPawn))
  (if Instant
    (Components|Movement|StopMovementImmediately (Pawn|GetMovementComponent (Variables|Default|GetOwnerPawn))))
  (Variables|Default|SetFinishedMovment true)
  (Variables|Default|SetDirectPathToTarget false)
  (Variables|Default|SetPreviousCheckDirectPathToTarget false)
  (Utilities|Array|Clear (Variables|Default|GetPath))
  (Variables|Default|SetLastPositionToMoveTo "0, 0, 0")
  (Default|CallMovementComplete))

(event Custom|MoveToRandomPosition
  (bind _ownerpawn (Variables|Default|GetOwnerPawn))
  (bind _returnvalue (Transformation|GetActorLocation _ownerpawn))
  (bind _nav_grid (CallFunction|EvaluateCurrentNavGrid _returnvalue _returnvalue))
  ;[1 1 1] Movement Commands
  (Utilities|IsValid _nav_grid
    (:Is%20Valid
      (CallFunction|MovetoNewPosition (Class|HeightNavigationVolume|GetRandomMovablePosition _nav_grid)))
    (:Is%20Not%20Valid
      (CallFunction|StopMovement true))))

(event EventBeginPlay
  ;[1 1 1] Setup
  (bind _aspawn (Utilities|Casting|CastToPawn (Components|GetOwner)))
  (bind _output_get (Variables|Default|SetOwnerPawn _aspawn))
  (Variables|Default|SetLastPositionToMoveTo (Transformation|GetActorLocation _output_get))
  (Variables|Default|SetpathCounter 0)
  (CallFunction|DirectPathLoop))

(event EventTick
  (params (DeltaSeconds :type Float%20%28single-precision%29))
  ;[1 1 1] Movement Loop
  (Utilities|FlowControl|Sequence
    (:then_0
      (if (not (Variables|Default|GetFinishedMovment))
        (if (Variables|Default|GetDirectPathToTarget)
          (Variables|Default|SetLastPositionToMoveTo (Variables|Default|GetTargetPosition))
          (if (CallFunction|IsBelowThreshold (Variables|Default|GetClosenessThreshold))
            (if (CallFunction|IsBelowThreshold 25.0)
              (Transformation|SetActorLocation (Variables|Default|GetOwnerPawn) (Variables|Default|GetLastPositionToMoveTo) false true)
              (CallFunction|StopMovement true)
              (else
                (CallFunction|MoveinDirection (Variables|Default|GetLastPositionToMoveTo) :!label _label)))
            (else
              (goto _label)))
          (elif (Variables|Default|GetPreviousCheckDirectPathToTarget)
            (CallFunction|MovetoNewPosition (Variables|Default|GetTargetPosition))
            (Variables|Default|SetPreviousCheckDirectPathToTarget false)
            (elif (CallFunction|IsBelowThreshold (Variables|Default|GetClosenessThreshold))
              (if (and (CallFunction|IsBelowThreshold 25.0) (>= (+ (Variables|Default|GetpathCounter) 1) (Utilities|Array|Length (Variables|Default|GetPath))))
                (Transformation|SetActorLocation (Variables|Default|GetOwnerPawn) (Variables|Default|GetLastPositionToMoveTo) false true)
                (CallFunction|StopMovement true)
                (else
                  (CallFunction|MoveinDirection (Variables|Default|GetLastPositionToMoveTo) :!label _label_2)
                  (if (CallFunction|IsBelowThreshold (Variables|Default|GetClosenessThreshold))
                    (if (not (>= (+ (Variables|Default|GetpathCounter) 1) (Utilities|Array|Length (Variables|Default|GetPath))))
                      (bind _result (Math|Integer|IncrementInt (Variables|Default|GetpathCounter))
                        (:%20%20
                          (Variables|Default|SetLastPositionToMoveTo (Utilities|Array|Get(acopy) (Variables|Default|GetPath) _result))))))))
              (else
                (goto _label_2)))))))
    (:then_1)))

(fn MoveinDirection
  (params (Position :type Vector))
  (if (Class|KismetMathLibrary|NotEqualExactlyVectorVector Position (Transformation|GetActorLocation (Variables|Default|GetOwnerPawn)))
    _
    (else
      _))
  (Pawn|Input|AddMovementInput (Variables|Default|GetOwnerPawn) (CallFunction|GetDirectionPosition Position) 1.0 false)
  (return))

(fn IsBelowThreshold
  (params (Threshold :type Float%20%28double-precision%29))
  (return (<= (Math|Vector|Distance(Vector) (Variables|Default|GetLastPositionToMoveTo) (Transformation|GetActorLocation (Variables|Default|GetOwnerPawn))) Threshold)))

(fn GetDirectionPosition
  (params (Position :type Vector))
  (return (Math|Vector|Normalize (- Position (Transformation|GetActorLocation (Variables|Default|GetOwnerPawn))))))

(fn GetNewPathtoPosition
  (params (Goal%20Position :type Vector))
  (bind _ownerpawn (Variables|Default|GetOwnerPawn))
  (bind _returnvalue (Transformation|GetActorLocation _ownerpawn))
  (bind _nav_grid (CallFunction|EvaluateCurrentNavGrid _returnvalue Goal%20Position))
  (Utilities|IsValid _nav_grid
    (:Is%20Valid
      (bind _path (Utilities|Paths|GetPath _nav_grid (Transformation|GetActorLocation (Variables|Default|GetOwnerPawn)) 0 Goal%20Position)
        (:Success
          (return _path true))
        (:Failed
          (return 0 false))))))

(fn EvaluateCurrentNavGrid
  (params (Start :type Vector) (Goal :type Vector))
  (bind _outactors (Actor|GetAllActorsOfClass "/Script/NavigationGrid.HeightNavigationVolume"))
  (bind _array_element (Utilities|Array|ForEachLoopwithBreak _outactors)
    (:LoopBody
      (bind _output_get (Variables|Default|SetNavMesh _array_element))
      (if (and (Class|HeightNavigationVolume|IsInsideVolume _output_get Start) (Class|HeightNavigationVolume|IsInsideVolume _output_get Goal))
        (return (Variables|Default|GetNavMesh))))
    (:Completed
      (return 0))))